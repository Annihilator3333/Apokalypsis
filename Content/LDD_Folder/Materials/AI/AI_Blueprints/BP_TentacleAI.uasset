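; Tentacle creature AI character that senses the player and drives its sound and material reactions.
; On BeginPlay it starts an attached squishy sound and loops a lurking-monster sound at random intervals.
; Seeing BP_FirstPersonCharacter sets blackboard "hasSeenPlayer?", clearing it after a delay before a timeline animates MP_TentacleCreature's "Amount".
; Any sighted pawn immediately triggers another "Amount" timeline and two DoOnce-throttled sounds.
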(event OnSeePawn(PawnSensing)
  (params (Pawn :type Pawn%20Object%20Reference))
  (bind _capsulecomponent (Variables|Collision|GetCapsuleComponent))
  (Utilities|FlowControl|Sequence
    (:then_0
      (Utilities|Casting|CastToBP_FirstPersonCharacter Pawn)
      (AI|Components|Blackboard|SetValueasBool (AI|GetBlackboard (AI|GetAIController self)) (Utilities|Name|MakeLiteralName "hasSeenPlayer?") true)
      (Utilities|FlowControl|Delay 5.0)
      (AI|Components|Blackboard|SetValueasBool (AI|GetBlackboard (AI|GetAIController self)) (Utilities|Name|MakeLiteralName "hasSeenPlayer?") false)
      (Rendering|Material|GetScalarParameterValue "/Game/LDD_Folder/Materials/MP_TentacleCreature.MP_TentacleCreature" "Amount" :!class /Script/Engine.KismetMaterialLibrary)
      (bind _newtrack_0 (Timeline|Timeline_3 PlayFromStart)
        (:Update
          (Rendering|Material|SetScalarParameterValue "/Game/LDD_Folder/Materials/MP_TentacleCreature.MP_TentacleCreature" "Amount" _newtrack_0 :!class /Script/Engine.KismetMaterialLibrary))))
    (:then_1
      (Rendering|Material|GetScalarParameterValue "/Game/LDD_Folder/Materials/MP_TentacleCreature.MP_TentacleCreature" "Amount" :!class /Script/Engine.KismetMaterialLibrary)
      (bind _newtrack_0_2 (Timeline|Timeline_4 PlayFromStart)
        (:Update
          (Rendering|Material|SetScalarParameterValue "/Game/LDD_Folder/Materials/MP_TentacleCreature.MP_TentacleCreature" "Amount" _newtrack_0_2 :!class /Script/Engine.KismetMaterialLibrary))))
    (:then_2
      (Utilities|FlowControl|DoOnce false :!label _label
        (:Completed
          (Audio|SpawnSoundAttached "/Game/LDD_Folder/Imported/Audio/creepy-hifreq-woosh-6873.creepy-hifreq-woosh-6873" _capsulecomponent "None" "0, 0, 0" "0, 0, 0" "KeepRelativeOffset" false 1.0 1.0 0.0 0 0)
          (Utilities|FlowControl|Delay 5.0)
          (goto _label Reset))))
    (:then_3
      (Utilities|FlowControl|DoOnce false :!label _label_2
        (:Completed
          (Audio|SpawnSoundAttached "/Game/LDD_Folder/Imported/Audio/WoodClicks/SC_WoodClicks.SC_WoodClicks" _capsulecomponent "None" "0, 0, 0" "0, 0, 0" "KeepRelativeOffset" false 1.0 1.0 0.0 0 0)
          (Utilities|FlowControl|Delay 2.0)
          (goto _label_2 Reset))))))

(event EventBeginPlay
  (Utilities|FlowControl|Sequence
    (:then_0
      (Utilities|FlowControl|Delay (Math|Random|RandomFloatinRange 15.0 45.0) :!label _label)
      (Audio|SpawnSoundAttached "/Game/LDD_Folder/Imported/Audio/halloween-horror-sound-lurking-monster-145070.halloween-horror-sound-lurking-monster-145070" (Variables|Collision|GetCapsuleComponent) "None" "0, 0, 0" "0, 0, 0" "KeepRelativeOffset" false 1.0 1.0 0.0 0 0)
      (Utilities|FlowControl|Delay 0.1)
      (goto _label))
    (:then_1
      (Audio|SpawnSoundAttached "/Game/LDD_Folder/Imported/Audio/squishy_flesh_thingy_seamless-30033.squishy_flesh_thingy_seamless-30033" (Variables|Collision|GetCapsuleComponent) "None" "0, 0, 0" "0, 0, 0" "KeepRelativeOffset" false 1.0 1.0 0.0 0 0))))

(event Collision|EventActorBeginOverlap
  (params (OtherActor :type Actor%20Object%20Reference)))

(fn ConstructionScript)