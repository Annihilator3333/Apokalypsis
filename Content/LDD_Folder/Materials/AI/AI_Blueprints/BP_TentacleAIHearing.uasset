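; Tentacle creature enemy that investigates sounds, reacts to seeing the player and plays looping idle audio.
; PawnSensing sight sets a Blackboard flag for five seconds and drives timelines on a material parameter collection to shift between transparent and solid.
; AIPerception stimuli from the player send it to the stimulus location; both senses trigger DoOnce-throttled chase sounds.
; Every Tick, a forward sphere trace damages whatever it hits.
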(event OnSeePawn(PawnSensing)
  (params (Pawn :type Pawn%20Object%20Reference))
  (bind _capsulecomponent (Variables|Collision|GetCapsuleComponent))
  ;[1 0.5098 0] AI Change Color and Play Audio On Chase
  (Utilities|FlowControl|Sequence
    (:then_0
      ;;[0.05259 0 0.3438] Change Color When Chasing
      (Utilities|Casting|CastToBP_FirstPersonCharacter Pawn)
      (AI|Components|Blackboard|SetValueasBool (AI|GetBlackboard (AI|GetAIController self)) (Utilities|Name|MakeLiteralName "hasSeenPlayer?") true)
      (Utilities|FlowControl|Delay 5.0)
      (AI|Components|Blackboard|SetValueasBool (AI|GetBlackboard (AI|GetAIController self)) (Utilities|Name|MakeLiteralName "hasSeenPlayer?") false)
      (Rendering|Material|GetScalarParameterValue "/Game/LDD_Folder/Materials/MP_TentacleCreature.MP_TentacleCreature" "Amount" :!class /Script/Engine.KismetMaterialLibrary)
      (bind _newtrack_0 (Timeline|Timeline_3 PlayFromStart)
        (:Update
          (Rendering|Material|SetScalarParameterValue "/Game/LDD_Folder/Materials/MP_TentacleCreature.MP_TentacleCreature" "Amount" _newtrack_0 :!class /Script/Engine.KismetMaterialLibrary) ; Set AI Either Transparent or Solid Depending on Amount Value
        )))
    (:then_1
      (Rendering|Material|GetScalarParameterValue "/Game/LDD_Folder/Materials/MP_TentacleCreature.MP_TentacleCreature" "Amount" :!class /Script/Engine.KismetMaterialLibrary)
      (bind _newtrack_0_2 (Timeline|Timeline_4 PlayFromStart)
        (:Update
          (Rendering|Material|SetScalarParameterValue "/Game/LDD_Folder/Materials/MP_TentacleCreature.MP_TentacleCreature" "Amount" _newtrack_0_2 :!class /Script/Engine.KismetMaterialLibrary) ; Set AI Either Transparent or Solid Depending on Amount Value
        )))
    (:then_2
      ;;[0 0.8873 1] Play Chase Sounds
      (Utilities|FlowControl|DoOnce false :!label _label
        (:Completed
          (Audio|SpawnSoundAttached "/Game/LDD_Folder/Imported/Audio/creepy-hifreq-woosh-6873.creepy-hifreq-woosh-6873" _capsulecomponent "None" "0, 0, 0" "0, 0, 0" "KeepRelativeOffset" false 1.0 1.0 0.0 0 0)
          (Utilities|FlowControl|Delay 5.0)
          (goto _label Reset))))
    (:then_3
      (Utilities|FlowControl|DoOnce false :!label _label_2
        (:Completed
          (Audio|SpawnSoundAttached "/Game/LDD_Folder/Imported/Audio/WoodClicks/SC_WoodClicks.SC_WoodClicks" _capsulecomponent "None" "0, 0, 0" "0, 0, 0" "KeepRelativeOffset" false 1.0 1.0 0.0 0 0)
          (Utilities|FlowControl|Delay 2.0)
          (goto _label_2 Reset))))))

(event OnTargetPerceptionUpdated(AIPerception)
  (params (Actor :type Actor%20Object%20Reference) (Stimulus :type AI%20Stimulus%20Structure))
  (bind (_age _expirationage _strength _stimuluslocation _receiverlocation _tag _bsuccessfullysensed) (Utilities|Struct|BreakAIStimulus Stimulus))
  (bind _capsulecomponent (Variables|Collision|GetCapsuleComponent))
  ;[1 0.5098 0] AI Move to Sound Location and Play Audio
  ;;[0.1042 0 1] AI Move To Location Of Heard Sound
  (Utilities|Casting|CastToBP_FirstPersonCharacter Actor)
  (if _bsuccessfullysensed
    (Variables|Default|SetInvestigating? true)
    (AI|AIMoveTo self _stimuluslocation 0 5.0 false
      (:then
        ;;[0 1 0.9848] AI Play Audio When Hearing Sound
        (Utilities|FlowControl|Sequence
          (:then_0
            (Utilities|FlowControl|DoOnce false :!label _label
              (:Completed
                (Audio|SpawnSoundAttached "/Game/LDD_Folder/Imported/Audio/creepy-hifreq-woosh-6873.creepy-hifreq-woosh-6873" _capsulecomponent "None" "0, 0, 0" "0, 0, 0" "KeepRelativeOffset" false 1.0 1.0 0.0 0 0)
                (Utilities|FlowControl|Delay 5.0)
                (goto _label Reset))))
          (:then_1
            (Utilities|FlowControl|DoOnce false :!label _label_2
              (:Completed
                (Audio|SpawnSoundAttached "/Game/LDD_Folder/Imported/Audio/WoodClicks/SC_WoodClicks.SC_WoodClicks" _capsulecomponent "None" "0, 0, 0" "0, 0, 0" "KeepRelativeOffset" false 1.0 1.0 0.0 0 0)
                (Utilities|FlowControl|Delay 2.0)
                (goto _label_2 Reset)))))))))

(event EventBeginPlay
  ;[0 0.7793 1] AI Idle Audio
  (Utilities|FlowControl|Sequence
    (:then_0
      (Utilities|FlowControl|Delay (Math|Random|RandomFloatinRange 15.0 45.0) :!label _label)
      (Audio|SpawnSoundAttached "/Game/LDD_Folder/Imported/Audio/halloween-horror-sound-lurking-monster-145070.halloween-horror-sound-lurking-monster-145070" (Variables|Collision|GetCapsuleComponent) "None" "0, 0, 0" "0, 0, 0" "KeepRelativeOffset" false 1.0 1.0 0.0 0 0)
      (Utilities|FlowControl|Delay 0.1)
      (goto _label))
    (:then_1
      (Audio|SpawnSoundAttached "/Game/LDD_Folder/Imported/Audio/squishy_flesh_thingy_seamless-30033.squishy_flesh_thingy_seamless-30033" (Variables|Collision|GetCapsuleComponent) "None" "0, 0, 0" "0, 0, 0" "KeepRelativeOffset" false 1.0 1.0 0.0 0 0))))

(event EventTick
  (params (DeltaSeconds :type Float%20%28single-precision%29))
  (bind _charactermovement (Variables|Character|GetCharacterMovement))
  (bind _updatedprimitive (Variables|/Script/Engine.MovementComponent|GetUpdatedPrimitive _charactermovement))
  (bind _returnvalue (Transformation|GetWorldLocation _updatedprimitive))
  ;[1 0 0] AI Damage Player
  (bind _outhit (Collision|SphereTraceByChannel _returnvalue (+ (* (Math|Vector|GetForwardVector (Variables|/Script/Engine.MovementComponent|GetUpdatedPrimitive _charactermovement)) (Variables|Default|GetHitRange)) _returnvalue) 5.0 "TraceTypeQuery1" false 0 "None"))
  (Game|Damage|ApplyDamage (.HitActor (Collision|BreakHitResult _outhit)) 1e+01 0 0) ; Damage Hit Player
)

(fn ConstructionScript)